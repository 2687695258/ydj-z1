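; BP_Feiyiche is a player-driven Chaos wheeled vehicle with a controllable arm, switchable cameras and a HUD.
; Input feeds the movement component and ABP_Feiyiche, which animates the lever, steering wheel and arm, with arm lowering blocked by ground contact.
; A CameraSwitcher cycles four spring-arm views with per-camera zoom limits.
; Tick drives exhaust from RPM and switches reverse, brake and turn lights through emissive alpha on dynamic materials.
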(event EventBeginPlay
  ;[1 1 1] 注释
  (Utilities|FlowControl|Sequence
    (:then_0
      (bind _asabp_feiyiche (Utilities|Casting|CastToABP_Feiyiche (Components|SkeletalMesh|GetAnimInstance (Variables|Character|GetMesh))))
      (Variables|Default|SetVehicleAnimBP _asabp_feiyiche))
    (:then_1
      (Default|SetCameras (Variables|Default|GetCameraSwitcher) (Utilities|Array|MakeArray (Variables|Default|GetOutsideCam) (Variables|Default|GetArmCam) (Variables|Default|GetWheelCam) (Variables|Default|GetInsideCam)))
      (Default|SetSpringArms (Variables|Default|GetCameraSwitcher) (Utilities|Array|MakeArray (Variables|Default|GetOutsideCamera) (Variables|Default|GetArmCamera) (Variables|Default|GetWheelCamera) (Variables|Default|GetInsideCamera)))
      (Default|SetSpringArmZoom (Variables|Default|GetCameraSwitcher) (Utilities|Array|MakeArray "50.000000,400.000000,1400.000000" "30.000000,50.000000,400.000000" "10.000000,30.000000,200.000000" "2.000000,15.000000,30.000000"))
      (Variables|/Game/CityColor/Blueprints/BP_CameraSwitcher_01_01.BP_CameraSwitcher_01_01_C|SetCurrentCamera (Variables|Default|GetCameraSwitcher) 1)
      (Default|ActivateNext (Variables|Default|GetCameraSwitcher)))
    (:then_2
      (CallFunction|SetupDynamicMaterials)
      (CallFunction|SetEmissiveonMaterial (Variables|Default|GetHeadLights) false)
      (CallFunction|SetEmissiveonMaterial (Variables|Default|GetStopLights) false)
      (CallFunction|SetEmissiveonMaterial (Variables|Default|GetReverseLights) false)
      (CallFunction|SetEmissiveonMaterial (Variables|Default|GetTurnLeftLight) false)
      (CallFunction|SetEmissiveonMaterial (Variables|Default|GetTurnRightLight) false)
      (CallFunction|SetEmissiveonMaterial (Variables|Default|GetPositionLight) false)
      (CallFunction|CreateVehicleUI)
      (Default|ToggleControls (Variables|Default|GetVehicleUI)))))

(event Collision|EventActorBeginOverlap
  (params (OtherActor :type Actor%20Object%20Reference)))

(event EventTick
  (params (DeltaSeconds :type Float%20%28single-precision%29))
  (Utilities|FlowControl|Sequence
    (:then_0
      (CallFunction|UpdateReverseGearEffects))
    (:then_1
      (默认|UpdateBrakeLights))
    (:then_2
      (CallFunction|UpdateTurnEffects))
    (:then_3
      (CallFunction|UpdateExhaustIntensity))))

(event Input|ActionEvents|InputActionCameraZoomin
  (params (Key :type Key%20Structure :default "None"))
  (bind _cameraswitcher (Variables|Default|GetCameraSwitcher))
  (bind _springarmzoom (Variables|/Game/CityColor/Blueprints/BP_CameraSwitcher_01_01.BP_CameraSwitcher_01_01_C|GetSpringArmZoom _cameraswitcher))
  (bind _currentcamera (Variables|/Game/CityColor/Blueprints/BP_CameraSwitcher_01_01.BP_CameraSwitcher_01_01_C|GetCurrentCamera _cameraswitcher))
  (bind _output (Utilities|Array|Get(acopy) _springarmzoom _currentcamera))
  ;[1 1 1] Camera zoom in/out
  (:Pressed
    (CallFunction|CameraZoom (- 0.0 (.x _output)) (.y _output) (.z _output) (Variables|/Game/CityColor/Blueprints/BP_CameraSwitcher_01_01.BP_CameraSwitcher_01_01_C|GetCurrentSpringArm (Variables|Default|GetCameraSwitcher)))))

(event Input|ActionEvents|InputActionJump
  (params (Key :type Key%20Structure :default "None"))
  (bind _vehiclemovementcomponent (Variables|Default|GetVehicleMovementComponent))
  ;[1 1 1] 载具移动
  (:Pressed
    (Class|ChaosVehicleMovementComponent|SetHandbrakeInput _vehiclemovementcomponent true)
    (Variables|Default|SetHandBrake true))
  (:Released
    (Class|ChaosVehicleMovementComponent|SetHandbrakeInput _vehiclemovementcomponent false)
    (Variables|Default|SetHandBrake false)))

(event Input|ActionEvents|InputActionToggleCamera
  (params (Key :type Key%20Structure :default "None"))
  ;[1 1 1] Camera toggle
  (:Pressed
    (Default|ActivateNext (Variables|Default|GetCameraSwitcher))))

(event Input|ActionEvents|InputActionCameraZoomOut
  (params (Key :type Key%20Structure :default "None"))
  (bind _cameraswitcher (Variables|Default|GetCameraSwitcher))
  (bind _springarmzoom (Variables|/Game/CityColor/Blueprints/BP_CameraSwitcher_01_01.BP_CameraSwitcher_01_01_C|GetSpringArmZoom _cameraswitcher))
  (bind _currentcamera (Variables|/Game/CityColor/Blueprints/BP_CameraSwitcher_01_01.BP_CameraSwitcher_01_01_C|GetCurrentCamera _cameraswitcher))
  (bind _output (Utilities|Array|Get(acopy) _springarmzoom _currentcamera))
  ;[1 1 1] Camera zoom in/out
  (:Pressed
    (CallFunction|CameraZoom (.x _output) (.y _output) (.z _output) (Variables|/Game/CityColor/Blueprints/BP_CameraSwitcher_01_01.BP_CameraSwitcher_01_01_C|GetCurrentSpringArm (Variables|Default|GetCameraSwitcher)))))

(event Input|ActionEvents|InputActionToggleLight
  (params (Key :type Key%20Structure :default "None"))
  (bind _downright (Variables|Default|GetDownRight))
  (bind _returnvalue (Rendering|IsVisible _downright))
  ;[1 1 1] 注释
  (:Released
    (Rendering|ToggleVisibility _downright false)
    (CallFunction|SetEmissiveonMaterial (Variables|Default|GetHeadLights) _returnvalue)
    (CallFunction|SetEmissiveonMaterial (Variables|Default|GetPositionLight) _returnvalue)))

(event Input|ActionEvents|InputActionOpenDoor
  (params (Key :type Key%20Structure :default "None"))
  (bind _mesh (Variables|Character|GetMesh))
  ;[1 1 1] Montage
  (:Pressed
    (Utilities|FlowControl|FlipFlop
      (:A
        (Animation|Montage|PlayMontage _mesh 0 0.5))
      (:B
        (Animation|Montage|PlayMontage _mesh 0 0.5)))))

(event Input|ActionEvents|InputActionToggleControls
  (params (Key :type Key%20Structure :default "None"))
  (:Pressed
    (Default|ToggleControls (Variables|Default|GetVehicleUI))))

(event Input|AxisEvents|InputAxisMoveForward
  (params (AxisValue :type Float%20%28single-precision%29))
  (bind _returnvalue (* AxisValue -1.0))
  (bind _vehiclemovementcomponent (Variables|Default|GetVehicleMovementComponent))
  (bind _vehicleanimbp (Variables|Default|GetVehicleAnimBP))
  ;[1 1 1] 载具移动
  (Class|ChaosVehicleMovementComponent|SetThrottleInput (Variables|Default|GetVehicleMovementComponent) AxisValue)
  (if (>= AxisValue 0.0)
    ;;[1 1 1] 类似于挂入倒挡，0是前进挡，1是倒挡
    (Class|ChaosVehicleMovementComponent|SetBrakeInput _vehiclemovementcomponent 0.0)
    (Default|UpdateMoveForwardLever _vehicleanimbp (* AxisValue -1.0) -14.0 26.0)
    (else
      (Class|ChaosVehicleMovementComponent|SetBrakeInput _vehiclemovementcomponent _returnvalue)
      (Default|UpdateMoveForwardLever _vehicleanimbp _returnvalue -14.0 26.0))))

(event Input|AxisEvents|InputAxisMoveRight
  (params (AxisValue :type Float%20%28single-precision%29))
  ;[1 1 1] 载具移动
  (Class|ChaosVehicleMovementComponent|SetSteeringInput (Variables|Default|GetVehicleMovementComponent) AxisValue)
  (Default|SetSteeringWheelInput (Variables|Default|GetVehicleAnimBP) AxisValue -1e+01 1e+01)
  (CallFunction|TurnLeftorRight AxisValue))

(event Input|AxisEvents|InputAxisTurn
  (params (AxisValue :type Float%20%28single-precision%29))
  ;[1 1 1] Camera rotation
  (Transformation|AddRelativeRotation (Variables|/Game/CityColor/Blueprints/BP_CameraSwitcher_01_01.BP_CameraSwitcher_01_01_C|GetCurrentSpringArm (Variables|Default|GetCameraSwitcher)) (Math|Rotator|MakeRotator 0.0 0.0 AxisValue) false false))

(event Input|AxisEvents|InputAxisLookUp
  (params (AxisValue :type Float%20%28single-precision%29))
  ;[1 1 1] Camera rotation
  (CallFunction|AddCameraPitchClamped (Variables|/Game/CityColor/Blueprints/BP_CameraSwitcher_01_01.BP_CameraSwitcher_01_01_C|GetCurrentSpringArm (Variables|Default|GetCameraSwitcher)) AxisValue -7e+01 0.0))

(event Input|AxisEvents|InputAxisArmSteering
  (params (AxisValue :type Float%20%28single-precision%29))
  (bind _vehicleanimbp (Variables|Default|GetVehicleAnimBP))
  (if (> AxisValue 0.0)
    (Default|AddArmInput _vehicleanimbp (* (Variables|Default|GetArmSpeedScale) AxisValue) 0.0 8e+01 :!label _label)
    (elif (not (Variables|Default|GetisGroundBlocked))
      (Utilities|IsValid _vehicleanimbp
        (:Is%20Valid
          (goto _label))))))

(fn ConstructionScript)

(fn CameraZoom
  (params (amount :type Float%20%28double-precision%29) (min :type Float%20%28double-precision%29) (max :type Float%20%28double-precision%29) (camera :type Spring%20Arm%20Component%20Object%20Reference))
  (Variables|/Script/Engine.SpringArmComponent|SetTargetArmLength camera (Math|Float|Clamp(Float) (+ amount (Variables|/Script/Engine.SpringArmComponent|GetTargetArmLength camera)) min max)))

(fn AddCameraPitchClamped
  (params (SpringArm :type Spring%20Arm%20Component%20Object%20Reference) (Value :type Float%20%28double-precision%29) (Min :type Float%20%28double-precision%29) (Max :type Float%20%28double-precision%29))
  (Transformation|AddRelativeRotation SpringArm (Math|Rotator|MakeRotator 0.0 (Math|Float|SelectFloat Value 0.0 (Math|Float|InRange(Float) (+ Value (.pitch (Transformation|GetWorldRotation SpringArm))) Min Max)) 0.0) false false))

(fn SetupDynamicMaterials
  (bind _mesh (Variables|Character|GetMesh))
  (Utilities|FlowControl|Sequence
    (:then_0
      (bind _returnvalue (Rendering|Material|CreateDynamicMaterialInstance _mesh 19 "/Game/CityColor/Material/MI_HeadLight.MI_HeadLight" "None" :!class /Script/Engine.PrimitiveComponent))
      (Variables|Default|SetHeadLights _returnvalue))
    (:then_1
      (bind _returnvalue_2 (Rendering|Material|CreateDynamicMaterialInstance _mesh 20 "/Game/CityColor/Material/MI_SpotLight.MI_SpotLight" "None" :!class /Script/Engine.PrimitiveComponent))
      (Variables|Default|SetStopLights _returnvalue_2))
    (:then_2
      (bind _returnvalue_3 (Rendering|Material|CreateDynamicMaterialInstance _mesh 67 "/Game/CityColor/Material/MI_ReasverLight.MI_ReasverLight" "None" :!class /Script/Engine.PrimitiveComponent))
      (Variables|Default|SetReverseLights _returnvalue_3))
    (:then_3
      (bind _returnvalue_4 (Rendering|Material|CreateDynamicMaterialInstance _mesh 6 "/Game/CityColor/Material/MI_TurnLight_ON.MI_TurnLight_ON" "None" :!class /Script/Engine.PrimitiveComponent))
      (Variables|Default|SetTurnLeftLight _returnvalue_4))
    (:then_4
      (bind _returnvalue_5 (Rendering|Material|CreateDynamicMaterialInstance _mesh 15 "/Game/CityColor/Material/MI_TurnLight_ON.MI_TurnLight_ON" "None" :!class /Script/Engine.PrimitiveComponent))
      (Variables|Default|SetTurnRightLight _returnvalue_5))
    (:then_5
      (bind _returnvalue_6 (Rendering|Material|CreateDynamicMaterialInstance _mesh 70 "/Game/CityColor/Material/MI_SpotLight.MI_SpotLight" "None" :!class /Script/Engine.PrimitiveComponent))
      (Variables|Default|SetPositionLight _returnvalue_6))))

(fn SetEmissiveonMaterial
  (params (Material :type Material%20Instance%20Dynamic%20Object%20Reference) (IsOn :type Boolean))
  (bind _returnvalue (Rendering|Material|GetVectorParameterValue Material (Variables|Default|GetEmissiveParameterName) :!class /Script/Engine.MaterialInstanceDynamic))
  (Rendering|Material|SetVectorParameterValue Material (Variables|Default|GetEmissiveParameterName) (Utilities|Struct|MakeLinearColor (.r _returnvalue) (.g _returnvalue) (.b _returnvalue) (select IsOn 1.0 0.0)) :!class /Script/Engine.MaterialInstanceDynamic))

(fn UpdateReverseGearEffects
  (CallFunction|SetEmissiveonMaterial (Variables|Default|GetReverseLights) (< (Class|ChaosVehicleMovementComponent|GetCurrentGear (Variables|Default|GetVehicleMovementComponent)) 0)))

(fn SetReverseLight
  (params (IsVisible :type Boolean))
  (if (Math|Boolean|NotEqual(Boolean) IsVisible (and (Variables|/Script/Engine.SceneComponent|GetbVisible (Variables|Default|GetRearLeft)) (Variables|/Script/Engine.SceneComponent|GetbVisible (Variables|Default|GetRearRight)))) ; When is changed
    (Rendering|SetVisibility (Variables|Default|GetRearLeft) IsVisible false)))

(fn UpdateBrakeLights
  (CallFunction|SetEmmisiveIntensityonMaterial (Variables|Default|GetStopLights) (select (or (Variables|Default|GetBrakeing) (Variables|Default|GetHandBrake)) 1.0 0.0)))

(fn SetEmmisiveIntensityonMaterial
  (params (Material :type Material%20Instance%20Dynamic%20Object%20Reference) (Intensity :type Float%20%28double-precision%29))
  (bind _returnvalue (Rendering|Material|GetVectorParameterValue Material (Variables|Default|GetEmissiveParameterName) :!class /Script/Engine.MaterialInstanceDynamic))
  (Rendering|Material|SetVectorParameterValue Material (Variables|Default|GetEmissiveParameterName) (Utilities|Struct|MakeLinearColor (.r _returnvalue) (.g _returnvalue) (.b _returnvalue) Intensity) :!class /Script/Engine.MaterialInstanceDynamic))

(fn TurnLeftorRight
  (params (AD :type Float%20%28double-precision%29))
  (Utilities|FlowControl|Sequence
    (:then_0
      (if (> AD 0.0)
        (Variables|Default|SetLeftOrRight 1)))
    (:then_1
      (if (< AD 0.0)
        (Variables|Default|SetLeftOrRight 2)))
    (:then_2
      (if (== AD 0.0)
        (Variables|Default|SetLeftOrRight 0)))))

(fn UpdateTurnEffects
  (Utilities|FlowControl|Sequence
    (:then_0
      (CallFunction|SetEmissiveonMaterial (Variables|Default|GetTurnLeftLight) (and (> (Math|Float|Truncate (Vehicle|GetForwardSpeed (Variables|Default|GetVehicleMovementComponent))) 0) (== (Variables|Default|GetLeftOrRight) 1))))
    (:then_1
      (CallFunction|SetEmissiveonMaterial (Variables|Default|GetTurnRightLight) (and (> (Math|Float|Truncate (Vehicle|GetForwardSpeed (Variables|Default|GetVehicleMovementComponent))) 0) (== (Variables|Default|GetLeftOrRight) 2))))
    (:then_2
      (if (== (Variables|Default|GetLeftOrRight) 0)
        (CallFunction|SetEmissiveonMaterial (Variables|Default|GetTurnLeftLight) false)
        (CallFunction|SetEmissiveonMaterial (Variables|Default|GetTurnRightLight) false)))))

(fn UpdateExhaustIntensity
  (Default|SetIntensity (Variables|Default|GetBP_VehicleExhaust_01_01) (Utilities|GetNormalizedRPM)))

(fn CreateVehicleUI
  (bind _returnvalue (UserInterface|CreateWidget "/Game/CityColor/Blueprints/B_HUDVehicle_01_01.B_HUDVehicle_01_01_C"))
  (bind _output_get (Variables|Default|SetVehicleUI _returnvalue))
  (UserInterface|Viewport|AddtoViewport _output_get 0))